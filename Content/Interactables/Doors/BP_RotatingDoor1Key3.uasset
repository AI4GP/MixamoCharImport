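; A rotating door Blueprint that an interacting instigator can open only when it holds a key.
; On Interaction it checks the instigator's HasKey1 flag, despite the Key3 in the asset name, and otherwise prints a locked message.
; A DoorRotation timeline adds yaw to the rotation cached at BeginPlay, zeroing roll and pitch.
; An IsDoorOpen flag makes opening one-way, with no close logic.
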(event EventBeginPlay
  (Variables|Default|SetInitialRotation (Transformation|GetActorRotation)))

(event EventInteraction
  (params (Instigator :type CH%20My%20Character%20Object%20Reference))
  (if (Variables|/Game/Characters/Player/CH_MyCharacter.CH_MyCharacter_C|GetHasKey1? Instigator)
    (if (not (Variables|Default|GetIsDoorOpen?))
      (Variables|Default|SetIsDoorOpen? true)
      (bind _rotation (Timeline|DoorRotation Play)
        (:Update
          (Transformation|SetActorRelativeRotation (Math|Rotator|MakeRotator 0.0 0.0 (+ _rotation (.Yaw (Math|Rotator|BreakRotator (Variables|Default|GetInitialRotation)))))))))
    (else
      (Development|PrintString "Door is Locked"))))

(fn ConstructionScript
  (|CallParentFunction))